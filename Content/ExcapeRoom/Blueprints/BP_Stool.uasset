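; BP_Stool is an escape-room stool that the player can pick up and drop through interaction.
; Interactwith toggles IsPickedUp, either attaching Cube1 in front of the first-person camera with physics off, or detaching it and re-enabling physics.
; LookAt supplies the "Pickup Stool" prompt, or removes tooltip widgets while held.
; MoveBox, not called here, instead positions the cube along the camera's forward vector and prints that location.
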(event `/Game/ExcapeRoom/Blueprints/BPI_Interact.InteractWith`
  (params (PlayerController :type "/Game/FirstPerson/Blueprints/BP_FirstPersonCharacter Object Reference"))
  (bind _cube1 (`self.Cube1`))
  (if (`self.IsPickedUp`)
    (`self.StartEndPickup` false)
    (`PrimitiveComponent.SetSimulatePhysics` _cube1 true)
    (`SceneComponent.K2_DetachFromComponent` (`self.Cube1`) "KeepWorld" "KeepRelative" "KeepRelative" true)
    (else
      (`self.StartEndPickup` true)
      (`PrimitiveComponent.SetSimulatePhysics` _cube1 false)
      (`SceneComponent.K2_AttachToComponent` _cube1 (`/Game/FirstPerson/Blueprints/BP_FirstPersonCharacter.FirstPersonCamera` PlayerController) "None" "KeepWorld" "KeepRelative" "KeepRelative" true)
      (`SceneComponent.K2_SetRelativeLocation` _cube1 (150.0 0.0 -25.0) false false))))

(event `OnInteract`)

(fn `LookAt`
  (returns (Verb :type Text) (Noun :type Text))
  (if (`self.IsPickedUp`)
    (bind _foundwidgets (`WidgetBlueprintLibrary.GetAllWidgetsOfClass` "/Game/ExcapeRoom/UserInterface/W_Tooltip.W_Tooltip_C"))
    (`Widget.RemoveFromParent` _foundwidgets)
    (else
      (return "Pickup" "Stool"))))

(fn `MoveBox`
  (params (`Player Controller` :type "/Game/FirstPerson/Blueprints/BP_FirstPersonCharacter Object Reference"))
  (bind _firstpersoncamera (`/Game/FirstPerson/Blueprints/BP_FirstPersonCharacter.FirstPersonCamera` `Player Controller`))
  (bind _returnvalue (+ (`SceneComponent.K2_GetComponentLocation` _firstpersoncamera) (* (`SceneComponent.GetForwardVector` _firstpersoncamera) 150.0)))
  (`SceneComponent.K2_SetWorldLocation` (`self.Cube1`) _returnvalue false false)
  (`KismetSystemLibrary.PrintString` (`KismetStringLibrary.Conv_VectorToString` _returnvalue)))

(fn `StartEndPickup`
  (params (SetState :type Boolean))
  (set `self.IsPickedUp` SetState))

(fn `UserConstructionScript`)