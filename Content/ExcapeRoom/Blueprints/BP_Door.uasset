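; BP_Door is an interactable escape-room door that can be locked behind a key item.
; Interacting while locked queries the player's inventory for KeyRequired, then either unlocks without opening or stays locked, showing a notice widget.
; Unlocked doors toggle open and closed through a Timeline-driven 90-degree rotation.
; LookAt returns verb and noun prompts based on whether KeyRequired is set, key possession and open state, ignoring the lock flag.
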(event `/Game/ExcapeRoom/Blueprints/BPI_Interact.InteractWith`
  (params (PlayerController :type "/Game/FirstPerson/Blueprints/BP_FirstPersonCharacter Object Reference"))
  (if (`self.IsLocked`)
    (bind _success (`/Game/ExcapeRoom/InventorySystem/BP_InventorySystem.QueryInventory` (`/Game/FirstPerson/Blueprints/BP_FirstPersonCharacter.BP_InventorySystem` PlayerController) (`self.KeyRequired`) 1))
    (if _success
      (`self.UnlockDoor`)
      (bind _returnvalue (`|CreateWidget` "/Game/ExcapeRoom/UserInterface/W_Notice.W_Notice_C" null "Door Unlocked"))
      (`UserWidget.AddToViewport` _returnvalue 0)
      (else
        (bind _returnvalue_2 (`|CreateWidget` "/Game/ExcapeRoom/UserInterface/W_Notice.W_Notice_C" null "Door Is Locked"))
        (`UserWidget.AddToViewport` _returnvalue_2 0)))
    (elif (`self.IsOpen`)
      (set `self.IsOpen` false)
      (`self.CloseDoor`)
      (else
        (set `self.IsOpen` true)
        (`self.OpenDoor`)))))

(event `OpenDoor`
  (if (not (`self.IsLocked`))
    (bind (_direction _rotation) (`Timeline|Timeline` :!label _label)
      (:`Update`
        (`SceneComponent.K2_SetRelativeRotation` (`self.Scene`) (`KismetMathLibrary.RLerp` (struct) (struct :`Yaw` 90.0) _rotation) false false)))))

(event `CloseDoor`
  (goto _label :!via `Reverse`))

(fn `LockDoor`
  (set `self.IsLocked` true))

(fn `LookAt`
  (returns (Verb :type Text) (Noun :type Text))
  (bind _keyrequired (`self.KeyRequired`)
    (:`then`
      (bind _asbp_first_person_character (cast `/Game/FirstPerson/Blueprints/BP_FirstPersonCharacter` (`Controller.K2_GetPawn` (`GameplayStatics.GetPlayerController` 0))))
      (bind _success (`/Game/ExcapeRoom/InventorySystem/BP_InventorySystem.QueryInventory` (`/Game/FirstPerson/Blueprints/BP_FirstPersonCharacter.BP_InventorySystem` _asbp_first_person_character) _keyrequired 1))
      (if _success
        (return "Unlock & Open" "Door")
        (else
          (return "Requires" (`/Game/ExcapeRoom/InventorySystem/Data/DA_Item.Name` _keyrequired)))))
    (:`else`
      (if (`self.IsOpen`)
        (return "Close" "Door")
        (else
          (return "Open" "Door"))))))

(fn `UnlockDoor`
  (set `self.IsLocked` false))

(fn `UserConstructionScript`)