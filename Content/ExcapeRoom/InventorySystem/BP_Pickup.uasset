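; BP_Pickup is an escape room pickup actor, configured by an item data asset that supplies its mesh, name and destroy-on-pickup flag.
; Interacting adds the item and quantity to the player controller's inventory component, then prints every content key.
; Inside that print loop, it destroys itself if the add succeeded and the asset allows it.
; LookAt returns a "Pickup" verb with the item name.
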(event `/Game/ExcapeRoom/Blueprints/BPI_Interact.InteractWith`
  (params (PlayerController :type "/Game/FirstPerson/Blueprints/BP_FirstPersonCharacter Object Reference"))
  (bind _dataasset (`self.DataAsset`))
  (bind _bp_inventorysystem (`/Game/FirstPerson/Blueprints/BP_FirstPersonCharacter.BP_InventorySystem` PlayerController))
  (bind _success (`/Game/ExcapeRoom/InventorySystem/BP_InventorySystem.AddToInventory` _bp_inventorysystem _dataasset (`self.Quantity`)))
  (bind _keys (`BlueprintMapLibrary.Map_Keys` (`/Game/ExcapeRoom/InventorySystem/BP_InventorySystem.Content` _bp_inventorysystem)))
  (for _array_element _keys
    (`KismetSystemLibrary.PrintString` (`KismetStringLibrary.Conv_ObjectToString` _array_element))
    (if (and _success (`/Game/ExcapeRoom/InventorySystem/Data/DA_Item.isDestroyedOnPickup` _dataasset))
      (`self.K2_DestroyActor`))))

(fn `LookAt`
  (returns (Verb :type Text) (Noun :type Text))
  (return "Pickup" (`/Game/ExcapeRoom/InventorySystem/Data/DA_Item.Name` (`self.DataAsset`))))

(fn `UserConstructionScript`
  (bind _dataasset (`self.DataAsset`)
    (:`then`
      (`StaticMeshComponent.SetStaticMesh` (`self.StaticMesh`) (`/Game/ExcapeRoom/InventorySystem/Data/DA_Item.StaticMesh` _dataasset)))
    (:`else`)))