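; BP_InventorySystem stores the items held in the escape room game as a map of item to quantity.
; AddToInventory increases an item's count and shows a notice widget, but skips unique items whose key already exists.
; RemoveFromInventory subtracts only when enough are held, leaving the key in the map.
; QueryInventory reports whether the key exists, regardless of requested quantity, along with its count.
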(fn `AddToInventory`
  (params (Item :type "/Game/ExcapeRoom/InventorySystem/Data/DA_Item Object Reference") (Quantity :type Integer))
  (returns (Success :type Boolean))
  (bind _success (`self.QueryInventory` Item Quantity))
  (if (not (and _success (`/Game/ExcapeRoom/InventorySystem/Data/DA_Item.IsUnique` Item)))
    (`BlueprintMapLibrary.Map_Add` (`self.Content`) (`local.Item`) (+ (`local.Quantity`) (`BlueprintMapLibrary.Map_Find` (`self.Content`) (`local.Item`))))
    (bind _returnvalue (`|CreateWidget` "/Game/ExcapeRoom/UserInterface/W_InventoryNotice.W_InventoryNotice_C" null (`|FormatText` "{itemname} Added to Inventory" (`/Game/ExcapeRoom/InventorySystem/Data/DA_Item.Name` (`local.Item`)))))
    (`UserWidget.AddToViewport` _returnvalue 0)
    (return true)))

(fn `QueryInventory`
  (params (Item :type "/Game/ExcapeRoom/InventorySystem/Data/DA_Item Object Reference") (Quantity :type Integer))
  (returns (Success :type Boolean) (Count :type Integer))
  (bind (_value _returnvalue) (`BlueprintMapLibrary.Map_Find` (`self.Content`) Item))
  (if _returnvalue
    (return true _value)
    (else
      (return false _value))))

(fn `RemoveFromInventory`
  (params (Item :type "/Game/ExcapeRoom/InventorySystem/Data/DA_Item Object Reference") (Quantity :type Integer))
  (bind _content (`self.Content`))
  (bind _value (`BlueprintMapLibrary.Map_Find` _content Item))
  (if (>= _value Quantity)
    (`BlueprintMapLibrary.Map_Add` _content Item (- _value Quantity))))